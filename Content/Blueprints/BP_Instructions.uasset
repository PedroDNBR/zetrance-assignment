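; Instruction display actor that shows step-by-step text on a WBP_Instructions widget and warns about items that are not microwave-safe.
; Next and Previus interact events step a bounded index through the Instructions array and refresh the text.
; Each Tick finds the first Microwave via GetAllActorsOfClass, showing the warning when its held actor's Type is Other.
; When that microwave is empty, Tick restores the current instruction.
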(event InteractDelegate(Previus)
  (if (> (Variables|Default|GetTextIndex) 0)
    (Math|Integer|DecrementInt (Variables|Default|GetTextIndex)
      (:%20%20
        (CallFunction|WriteMessageinScreen)))))

(event InteractDelegate(Next)
  (if (< (Variables|Default|GetTextIndex) (- (Utilities|Array|Length (Variables|Default|GetInstructions)) 1))
    (Math|Integer|IncrementInt (Variables|Default|GetTextIndex)
      (:%20%20
        (CallFunction|WriteMessageinScreen)))))

(event EventBeginPlay
  (CallFunction|WriteMessageinScreen))

(event Collision|EventActorBeginOverlap
  (params (OtherActor :type Actor%20Object%20Reference)))

(event EventTick
  (params (DeltaSeconds :type Float%20%28single-precision%29))
  (bind _outactors (Actor|GetAllActorsOfClass "/Script/ZetranceTest.Microwave"))
  (Utilities|IsValid (Utilities|Array|Get(acopy) _outactors)
    (:Is%20Valid
      (Utilities|IsValid (Variables|/Script/ZetranceTest.Microwave|GetActorInTheMicrowave (Utilities|Array|Get(acopy) _outactors))
        (:Is%20Valid
          (if (Utilities|Enum|Equal(Enum) (Variables|/Script/ZetranceTest.Grabbable|GetType (Variables|/Script/ZetranceTest.Microwave|GetActorInTheMicrowave (Utilities|Array|Get(acopy) _outactors))) "ET_Other")
            (CallFunction|WriteWarningMessage)))
        (:Is%20Not%20Valid
          (CallFunction|WriteMessageinScreen))))))

(fn ConstructionScript)

(fn WriteMessageinScreen
  (bind _aswbp_instructions (Utilities|Casting|CastToWBP_Instructions (UserInterface|GetWidget (Variables|Default|GetWidget))))
  (Default|UpdateInstructions _aswbp_instructions (Utilities|Array|Get(acopy) (Variables|Default|GetInstructions) (Variables|Default|GetTextIndex))))

(fn WriteWarningMessage
  (bind _aswbp_instructions (Utilities|Casting|CastToWBP_Instructions (UserInterface|GetWidget (Variables|Default|GetWidget))))
  (Default|UpdateInstructions _aswbp_instructions (Variables|Default|GetNotMicrowaveSaveAlertMessage)))